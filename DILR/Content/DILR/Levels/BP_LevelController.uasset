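; BP_LevelController builds a procedural level out of BP_Room actors, adding one room per CreateRoom call.
; It picks random spawnpoints, line-tracing vertically through each on the Visibility channel and discarding blocked ones until one is clear.
; The spawned room is recorded and its own spawnpoints join the candidate pool, so the layout can grow outward, with a running room count.
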(fn ConstructionScript)

(fn CreateRoom
  (while (LocalVariables|GetHit)
    (bind _output_get (LocalVariables|SetSpawnpoint (.OutItem (Utilities|Array|Random (Variables|Default|GetSpawnpoints)))))
    (bind _returnvalue (Collision|LineTraceByChannel (Math|Vector|MakeVector (.X (Math|Vector|BreakVector (Transformation|GetWorldLocation _output_get))) (.Y (Math|Vector|BreakVector (Transformation|GetWorldLocation _output_get))) (+ (.Z (Math|Vector|BreakVector (Transformation|GetWorldLocation _output_get))) 5e+02)) (Math|Vector|MakeVector (.X (Math|Vector|BreakVector (Transformation|GetWorldLocation _output_get))) (.Y (Math|Vector|BreakVector (Transformation|GetWorldLocation _output_get))) (- (.Z (Math|Vector|BreakVector (Transformation|GetWorldLocation _output_get))) 5e+02)) "TraceTypeQuery1" false 0 "None"))
    (if _returnvalue
      (Utilities|Array|RemoveItem (Variables|Default|GetSpawnpoints) (LocalVariables|GetSpawnpoint))
      (else
        (LocalVariables|SetHit false))))
  (bind _returnvalue_2 (Game|SpawnActorfromClass "/Game/DILR/Blueprints/Rooms/BP_Room.BP_Room_C" (Transformation|GetWorldTransform (LocalVariables|GetSpawnpoint)) "Undefined" "MultiplyWithRoot" 0 0))
  (Utilities|Array|Add (Variables|Default|GetRooms) _returnvalue_2)
  (bind _children (Default|GetSpawnpoints _returnvalue_2))
  (for _array_element _children
    (Utilities|Array|Add (Variables|Default|GetSpawnpoints) _array_element))
  (Variables|Default|SetCurrentRoomNumber (+ (Variables|Default|GetCurrentRoomNumber) 1)))