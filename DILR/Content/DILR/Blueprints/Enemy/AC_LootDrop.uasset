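; AC_LootDrop is an enemy loot component that spawns a weighted-random collectible at a given drop location.
; DropLoot passes a roll between 0 and 1 to RandItem, which walks the DropList data table while summing each row's Chance.
; The first row whose cumulative chance reaches the roll spawns a BP_Collectible carrying that item, so at most one drops per roll.
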(fn DropLoot
  (params (DropLocation :type Transform))
  ;[0.15 0.15 0.15 0.5] Randomly select an item from the array to spawn
  (CallFunction|RandItem (Math|Random|RandomFloatinRange 0.0 1.0) DropLocation))

(fn RandItem
  (params (Chance :type Float%20%28double-precision%29) (Location :type Transform))
  (bind _outrownames (DataTable|GetDataTableRowNames (Variables|Default|GetDropList)))
  (bind _array_element (Utilities|Array|ForEachLoopwithBreak _outrownames :!label _label)
    (:LoopBody
      (bind _returnvalue (Utilities|GetDataTableRow (Variables|Default|GetDropList) _array_element)
        (:then
          (bind _output_get (LocalVariables|SetItem _returnvalue))
          ;[0.15 0.15 0.15 0.5] Is this item chosen ?
          (bind _output_get_2 (LocalVariables|SetCumulativeProcentage (+ (Utilities|Struct|BreakF_LootDrop _output_get) (LocalVariables|GetCumulativeProcentage))))
          (if (<= Chance _output_get_2)
            ;[0.15 0.15 0.15 0.5] Spawn item at location
            (bind _returnvalue_2 (Game|SpawnActorfromClass "/Game/DILR/Blueprints/Items/BP_Collectible.BP_Collectible_C" Location "Undefined" "MultiplyWithRoot" 0 (Utilities|Struct|BreakF_LootDrop (LocalVariables|GetItem)) 0))
            (LocalVariables|SetCollectibleItem _returnvalue_2)
            (goto _label Break)))))
    (:Completed
      (return (LocalVariables|GetCollectibleItem)))))