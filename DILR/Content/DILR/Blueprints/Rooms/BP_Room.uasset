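; BP_Room is a room actor that manages four door child actors and the spawn points they provide.
; SetupDoors queries each door through an interface message and stores the openable ones in DoorsList.
; ActivateDoors toggles those doors by negating their world Z position, which mirrors them across the Z=0 plane.
; GetSpawnpoints gathers a spawn point from all four doors by interface message and returns the accumulated list.
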(fn ConstructionScript)

(fn GetSpawnpoints
  (for _array_element (Utilities|Array|MakeArray (Variables|Default|GetDoor0) (Variables|Default|GetDoor1) (Variables|Default|GetDoor2) (Variables|Default|GetDoor3))
    (bind _spawnpoint (Class|BIDoor|GetSpawnpoint(Message) (Variables|/Script/Engine.ChildActorComponent|GetChildActor _array_element)))
    (Utilities|Array|Add (LocalVariables|GetSpawnpoints) _spawnpoint))
  (return (LocalVariables|GetSpawnpoints)))

(fn ActivateDoors
  (for _array_element (Variables|Default|GetDoorsList)
    (Transformation|SetWorldLocation _array_element (Math|Vector|MakeVector (.X (Math|Vector|BreakVector (Transformation|GetWorldLocation _array_element))) (.Y (Math|Vector|BreakVector (Transformation|GetWorldLocation _array_element))) (* (.Z (Math|Vector|BreakVector (Transformation|GetWorldLocation _array_element))) -1.0)) false false)))

(fn SetupDoors
  (for _array_element (Utilities|Array|MakeArray (Variables|Default|GetDoor0) (Variables|Default|GetDoor1) (Variables|Default|GetDoor2) (Variables|Default|GetDoor3))
    (bind _can (Class|BIDoor|CanIOpen(Message) (Variables|/Script/Engine.ChildActorComponent|GetChildActor _array_element)))
    (if _can
      (Utilities|Array|Add (Variables|Default|GetDoorsList) _array_element))))