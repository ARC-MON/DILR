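; Door Blueprint for rooms that exposes a spawnpoint component and reports whether the door can open.
; CanIOpen runs a vertical Visibility line trace through the spawnpoint, from above it to below it, and returns true when anything blocks the trace.
; GetSpawnpoint hands that component to callers; the door holds no opening or spawning logic in these graphs.
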(fn ConstructionScript)

(fn CanIOpen
  (bind _spawnpoint (Variables|Default|GetSpawnpoint))
  (bind _returnvalue (Transformation|GetWorldLocation _spawnpoint))
  (bind (_x _y _z) (Math|Vector|BreakVector _returnvalue))
  (bind (_x_2 _y_2 _z_2) (Math|Vector|BreakVector _returnvalue))
  (bind _returnvalue_2 (Collision|LineTraceByChannel (Math|Vector|MakeVector _x _y (+ _z 5e+02)) (Math|Vector|MakeVector _x_2 _y_2 (- _z_2 5e+02)) "TraceTypeQuery1" false 0 "None"))
  (return _returnvalue_2))

(fn GetSpawnpoint
  (return (Variables|Default|GetSpawnpoint)))