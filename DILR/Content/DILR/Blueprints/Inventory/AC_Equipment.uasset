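; Equipment component that manages a three-slot weapon loadout for its owner, storing each weapon's item data in a map keyed by slot index.
; EquipItem spawns a gun component on the WeaponSocket of Attach and colors it by rarity from the game instance.
; Using the weapon passes in the active slot's stats and tags, and weapon update events write changes back.
; Index changes wrap around, and deequipping the active slot messages the owner.
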(fn EquipItem
  ;[0.15 0.15 0.15 0.5] Is there where to place weapon
  (Utilities|IsValid (Variables|Default|GetAttach)
    (:Is%20Valid
      ;[0.15 0.15 0.15 0.5] Is there weapon to equip
      (if (.ReturnValue (Utilities|Map|Find (Variables|Default|GetWeapons) (Variables|Default|GetActiveIndex)))
        ;[0.15 0.15 0.15 0.5] Create weapon
        (bind _returnvalue (Game|AddComponentbyClass (Components|GetOwner) "/Game/DILR/Blueprints/Items/Weapons/SKC_BasicGun.SKC_BasicGun_C" false))
        (Variables|Default|SetActiveWeapon _returnvalue)
        ;[0.15 0.15 0.15 0.5] Set weapon color
        (CallFunction|SetMaterial)
        ;[0.15 0.15 0.15 0.5] Update weapon in inventory if something happens
        (EventDispatchers|BindEventtoUpdateStats (Variables|Default|GetActiveWeapon) (EventDispatchers|CreateEvent :!event UpdateActiveStats))
        (EventDispatchers|BindEventtoUpdateTags (Variables|Default|GetActiveWeapon) (EventDispatchers|CreateEvent :!event UpdateActiveTags))
        ;[0.15 0.15 0.15 0.5] Attach weapon to designated place
        (Transformation|AttachComponentToComponent (Variables|Default|GetActiveWeapon) (Variables|Default|GetAttach) "WeaponSocket" "KeepRelative" "KeepRelative" "KeepRelative" true)))))

(fn UpdateWeapon
  (params (Index :type Integer) (Item :type BDA%20Item%20Object%20Reference) (Rarity :type E_Rarity%20Enum :default "NewEnumerator0") (Quantity :type Integer) (Stats :type Map%20of%20E_ItemStats%20Enums%20to%20Reals :default "NewEnumerator0") (Tags :type Gameplay%20Tag%20Container%20Structure))
  (Utilities|Map|Add (Variables|Default|GetWeapons) Index (Utilities|Struct|MakeF_InventoryItem Item Rarity Quantity Stats Tags)))

(fn RemoveWeapon
  (params (Index :type Integer))
  (Utilities|Map|Remove (Variables|Default|GetWeapons) Index))

(fn ChangeActiveIndex
  (params (Amount :type Integer))
  ;[0.15 0.15 0.15 0.5] Change index by number
  (LocalVariables|SetNewIndex (- (Variables|Default|GetActiveIndex) Amount))
  ;[0.15 0.15 0.15 0.5] Set index base of possible weapon number
  (if (< (LocalVariables|GetNewIndex) 0)
    (Variables|Default|SetActiveIndex 2)
    (elif (> (LocalVariables|GetNewIndex) 2)
      (Variables|Default|SetActiveIndex 0)
      (else
        (Variables|Default|SetActiveIndex (LocalVariables|GetNewIndex))))))

(fn EquipifActive
  (params (Index :type Integer))
  (if (== Index (Variables|Default|GetActiveIndex))
    (CallFunction|EquipItem)))

(fn UseActiveWeapon
  (params (Target :type Vector))
  (bind _weapons (Variables|Default|GetWeapons))
  (bind _activeindex (Variables|Default|GetActiveIndex))
  (bind _value (Utilities|Map|Find _weapons _activeindex))
  (bind (_stats _tags) (Utilities|Struct|BreakF_InventoryItem _value))
  ;[0.15 0.15 0.15 0.5] If there is weapon
  (Utilities|IsValid (Variables|Default|GetActiveWeapon)
    (:Is%20Valid
      ;[0.15 0.15 0.15 0.5] Use weapon with stats and tags on target
      (Default|UseWeapon (Variables|Default|GetActiveWeapon) Target _stats _tags))))

(fn UpdateActiveStats
  (params (Stats :type Map%20of%20E_ItemStats%20Enums%20to%20Reals :default "NewEnumerator0"))
  (bind _weapons (Variables|Default|GetWeapons))
  (bind _activeindex (Variables|Default|GetActiveIndex))
  (bind _value (Utilities|Map|Find _weapons _activeindex))
  (bind (_itemdataasset _rarity _quantity _tags) (Utilities|Struct|BreakF_InventoryItem _value))
  (Utilities|Map|Add (Variables|Default|GetWeapons) (Variables|Default|GetActiveIndex) (Utilities|Struct|MakeF_InventoryItem _itemdataasset _rarity _quantity Stats _tags)))

(fn UpdateActiveTags
  (params (Tags :type Gameplay%20Tag%20Container%20Structure))
  (bind _weapons (Variables|Default|GetWeapons))
  (bind _activeindex (Variables|Default|GetActiveIndex))
  (bind _value (Utilities|Map|Find _weapons _activeindex))
  (bind (_itemdataasset _rarity _quantity _stats) (Utilities|Struct|BreakF_InventoryItem _value))
  (Utilities|Map|Add (Variables|Default|GetWeapons) (Variables|Default|GetActiveIndex) (Utilities|Struct|MakeF_InventoryItem _itemdataasset _rarity _quantity _stats Tags)))

(fn DeequipifActive
  (params (Index :type Integer))
  (if (== Index (Variables|Default|GetActiveIndex))
    (Class|BIPlayer|DropChild(Message) (Components|GetOwner))))

(fn SetMaterial
  (bind _asgi_dilrgame_instance (Utilities|Casting|CastToGI_DILRGameInstance (Game|GetGameInstance)))
  (Rendering|Material|SetMaterial (Variables|Default|GetActiveWeapon) 0 (Utilities|Struct|BreakF_Rarity (.Value (Utilities|Map|Find (Variables|/Game/DILR/GameInstance/GI_DILRGameInstance.GI_DILRGameInstance_C|GetRarity _asgi_dilrgame_instance) (Utilities|Struct|BreakF_InventoryItem (.Value (Utilities|Map|Find (Variables|Default|GetWeapons) (Variables|Default|GetActiveIndex)))))))))