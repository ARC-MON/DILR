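; Base enemy character that wires health, equipment and player sensing together for an AI-controlled opponent.
; On spawn it binds a dying event intended for item drops, equips its weapon on the mesh and fills the health bar.
; Damage goes through the HP component and refreshes the bar.
; Pawn sensing sets blackboard visibility, with a retriggerable one-second delay clearing visibility and weapon-range flags once sightings stop.
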(event OnSeePawn(PawnSensing)
  (params (Pawn :type Pawn%20Object%20Reference))
  (Utilities|FlowControl|Sequence
    (:then_0
      ;[0.15 0.15 0.15 0.5] If player detected chabge variable in blackbord
      (AI|Components|Blackboard|SetValueasBool (AI|GetBlackboard (AI|GetAIController self)) (Utilities|Name|MakeLiteralName "PlayerVisible") true))
    (:then_1
      ;[0.15 0.15 0.15 0.5] If player was not seen for 1 second return to roaming
      (Utilities|FlowControl|RetriggerableDelay 1.0)
      (AI|Components|Blackboard|SetValueasBool (AI|GetBlackboard (AI|GetAIController self)) (Utilities|Name|MakeLiteralName "PlayerVisible") false)
      (AI|Components|Blackboard|SetValueasBool (AI|GetBlackboard (AI|GetAIController self)) (Utilities|Name|MakeLiteralName "PlayerInWeaponRange") false))))

(event EventBeginPlay
  (bind _ac_hpsystem (Variables|Default|GetAC_HpSystem))
  ;[0.15 0.15 0.15 0.5] To drop items when dead
  (EventDispatchers|BindEventtoDying (Variables|Default|GetAC_HpSystem) (EventDispatchers|CreateEvent (Variables|Default|GetAC_LootDrop) :!event DropLoot))
  ;[0.15 0.15 0.15 0.5] Place for weapon
  (Variables|/Game/DILR/Blueprints/Inventory/AC_Equipment.AC_Equipment_C|SetAttach (Variables|Default|GetAC_Equipment) (Variables|Character|GetMesh))
  ;[0.15 0.15 0.15 0.5] Equip weapon
  (Default|EquipItem (Variables|Default|GetAC_Equipment))
  ;[0.15 0.15 0.15 0.5] Set hp bar value
  (Class|BIEnemyHP|SetHp(Message) (Variables|Default|GetHealth) (Variables|/Game/DILR/Blueprints/Characters/AC_HpSystem.AC_HpSystem_C|GetCurrentHP _ac_hpsystem) (Variables|/Game/DILR/Blueprints/Characters/AC_HpSystem.AC_HpSystem_C|GetMaxHp _ac_hpsystem)))

(event Game|Damage|EventAnyDamage
  (params (Damage :type Float%20%28single-precision%29) (DamageType :type Damage%20Type%20Object%20Reference) (InstigatedBy :type Controller%20Object%20Reference) (DamageCauser :type Actor%20Object%20Reference))
  (bind _ac_hpsystem (Variables|Default|GetAC_HpSystem))
  ;[0.15 0.15 0.15 0.5] Take damage
  (Default|TakeDamage (Variables|Default|GetAC_HpSystem) Damage)
  ;[0.15 0.15 0.15 0.5] Update hp bar
  (Class|BIEnemyHP|SetHp(Message) (Variables|Default|GetHealth) (Variables|/Game/DILR/Blueprints/Characters/AC_HpSystem.AC_HpSystem_C|GetCurrentHP _ac_hpsystem) (Variables|/Game/DILR/Blueprints/Characters/AC_HpSystem.AC_HpSystem_C|GetMaxHp _ac_hpsystem)))

(fn ConstructionScript)