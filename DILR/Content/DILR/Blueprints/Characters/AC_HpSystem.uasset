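; AC_HpSystem is an actor component that tracks hit points for the actor that owns it.
; On BeginPlay it fills current HP to the maximum.
; TakeDamage subtracts damage and fires an HP update event with current and max values.
; When HP reaches zero or below, it fires a dying event and destroys the owner.
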(event EventBeginPlay
  ;[0.15 0.15 0.15 0.5] When spawn set hp to max hp value
  (Variables|Default|SetCurrentHP (Variables|Default|GetMaxHp)))

(fn TakeDamage
  (params (Damage :type Float%20%28double-precision%29))
  ;[0.15 0.15 0.15 0.5] Take damage and trigger event
  (bind _output_get (Variables|Default|SetCurrentHP (- (Variables|Default|GetCurrentHP) Damage)))
  (Default|CallUpdateHP _output_get (Variables|Default|GetMaxHp))
  ;[0.15 0.15 0.15 0.5] If HP is lower or equal 0 trigger dying event and destroy owner
  (if (<= (Variables|Default|GetCurrentHP) 0.0)
    (Default|CallDying)
    (Actor|DestroyActor (Components|GetOwner))))