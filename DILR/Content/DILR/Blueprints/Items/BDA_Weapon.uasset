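; BDA_Weapon is a weapon item Blueprint that exposes its combat stats as a map.
; GetStatsMap fills WeaponStats with damage, accuracy, rate of fire, reload speed and ammunition, each keyed by an enum entry, then returns it.
; Ammunition is converted to a double so it shares the map's value type with the other stats.
; The function adds to the WeaponStats variable without clearing it first.
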(fn GetStatsMap
  (Utilities|Map|Add (LocalVariables|GetWeaponStats) "NewEnumerator0" (Variables|Default|GetDamage))
  (Utilities|Map|Add (LocalVariables|GetWeaponStats) "NewEnumerator1" (Variables|Default|GetAccuracy))
  (Utilities|Map|Add (LocalVariables|GetWeaponStats) "NewEnumerator2" (Variables|Default|GetRateOfFire))
  (Utilities|Map|Add (LocalVariables|GetWeaponStats) "NewEnumerator3" (Variables|Default|GetReloadSpeed))
  (Utilities|Map|Add (LocalVariables|GetWeaponStats) "NewEnumerator4" (Math|Conversions|ToFloat(Integer) (Variables|Default|GetAmmunition)))
  (return (LocalVariables|GetWeaponStats)))